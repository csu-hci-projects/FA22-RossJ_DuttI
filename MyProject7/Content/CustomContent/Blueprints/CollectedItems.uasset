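; Tracker for five collectible items that signals an opened door once every one is collected.
; Each Collect function swaps its button's material to the collected look, sets that item's flag and returns the button.
; Tick polls the five flags and calls the ShowDoorOpened dispatcher on every frame while all are true.
; The ShowDoorOpened_Event handler makes the text render visible; its binding is not in these graphs.
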(event `self.ReceiveTick`
  (params (DeltaSeconds :type "Float (single-precision)"))
  (if (`self.Collected1`)
    (if (`self.Collected2`)
      (if (`self.Collected3`)
        (if (`self.Collected4`)
          (if (`self.Collected5`)
            (`self.Show Door Opened`)))))))

(event `Show Door Opened_Event`
  (`SceneComponent.SetVisibility` (`self.TextRender`) true false))

(fn `Collect1`
  (returns (Button1 :type "MeshComponent Object Reference"))
  (bind _button1 (`self.Button1`))
  (`PrimitiveComponent.SetMaterial` _button1 0 "/Game/CustomContent/Materials/Collected.Collected")
  (set `self.Collected1` true)
  (return _button1))

(fn `Collect2`
  (returns (`Button 2` :type "MeshComponent Object Reference"))
  (bind _button2 (`self.Button2`))
  (`PrimitiveComponent.SetMaterial` _button2 0 "/Game/CustomContent/Materials/Collected.Collected")
  (set `self.Collected2` true)
  (return _button2))

(fn `Collect3`
  (returns (`Button 3` :type "MeshComponent Object Reference"))
  (bind _button3 (`self.Button3`))
  (`PrimitiveComponent.SetMaterial` _button3 0 "/Game/CustomContent/Materials/Collected.Collected")
  (set `self.Collected3` true)
  (return _button3))

(fn `Collect4`
  (returns (`Button 4` :type "MeshComponent Object Reference"))
  (bind _button4 (`self.Button4`))
  (`PrimitiveComponent.SetMaterial` _button4 0 "/Game/CustomContent/Materials/Collected.Collected")
  (set `self.Collected4` true)
  (return _button4))

(fn `Collect5`
  (returns (`Button 5` :type "MeshComponent Object Reference"))
  (bind _button5 (`self.Button5`))
  (`PrimitiveComponent.SetMaterial` _button5 0 "/Game/CustomContent/Materials/Collected.Collected")
  (set `self.Collected5` true)
  (return _button5))

(fn `UserConstructionScript`)