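; VR grab-triggered actor that starts one of the randomly chosen large levels, presumably the hard tier going by the asset name.
; When grabbed, it builds a LargeLevel name from a random number and opens that level.
; Before opening, GetLevelName maps that name through parallel LevelNumbers and LevelNames arrays, falling back to the raw name, and the result is appended to VR_GameInstance's LevelNames.
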(event `self.GrabComponent.OnGrabbed`
  ;[0 0 0] Gets random level name and adds it name to the list of level names in game instance
  (bind _result (`/Engine/EditorBlueprintResources/StandardMacros.IncrementInt` (`KismetMathLibrary.RandomInteger` 3))
    (:`  `
      (bind _asvr_game_instance (cast `/Game/CustomContent/Blueprints/VR_GameInstance` (`GameplayStatics.GetGameInstance`)))
      (bind _returnvalue (`KismetStringLibrary.Concat_StrStr` "LargeLevel" (`KismetStringLibrary.Conv_IntToString` _result)))
      (bind _levelname (`self.Get Level Name` _returnvalue))
      (`KismetArrayLibrary.Array_Add` (`/Game/CustomContent/Blueprints/VR_GameInstance.LevelNames` _asvr_game_instance) _levelname)
      (`GameplayStatics.OpenLevel` (`KismetStringLibrary.Conv_StringToName` _returnvalue)))))

(fn `Get Level Name`
  (params (LevelNumber :type String))
  (returns (LevelName :type Name))
  (locals (LevelNames :type "Array of Name") (LevelNumbers :type "Array of String"))
  (for (_array_element _array_index) (`local.LevelNumbers`)
    (if (`KismetStringLibrary.EqualEqual_StrStr` _array_element LevelNumber)
      (return (`|GetArrayItem` (`local.LevelNames`) _array_index))))
  (return (`KismetStringLibrary.Conv_StringToName` LevelNumber)))

(fn `UserConstructionScript`)